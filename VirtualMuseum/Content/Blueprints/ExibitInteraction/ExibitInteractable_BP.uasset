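; Exhibit interactable actor that shows a configurable widget on screen while something overlaps it.
; The construction script adds a box collider placed and sized by the Collider and ColliderSize variables.
; Overlap begin clears existing top-level widgets of that class and adds a new one to the viewport.
; Overlap end removes them after a short delay, with DoOnce gates resetting after each pass and no filter on the overlapping actor.
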(event `self.ReceiveActorBeginOverlap`
  (params (OtherActor :type "Actor Object Reference"))
  (bind _widget (`self.Widget`))
  (`/Engine/EditorBlueprintResources/StandardMacros.DoOnce` false :!label _label
    (:`Completed`
      (bind _foundwidgets (`WidgetBlueprintLibrary.GetAllWidgetsOfClass` _widget))
      (`Widget.RemoveFromParent` _foundwidgets)
      (bind _returnvalue (`|CreateWidget` _widget))
      (`UserWidget.AddToViewport` _returnvalue 0)
      (goto _label :!via `Reset`))))

(event `self.ReceiveActorEndOverlap`
  (params (OtherActor :type "Actor Object Reference"))
  (`/Engine/EditorBlueprintResources/StandardMacros.DoOnce` false :!label _label_2
    (:`Completed`
      (`KismetSystemLibrary.Delay` 1.0)
      (bind _foundwidgets (`WidgetBlueprintLibrary.GetAllWidgetsOfClass` (`self.Widget`)))
      (`Widget.RemoveFromParent` _foundwidgets)
      (goto _label_2 :!via `Reset`))))

(fn `UserConstructionScript`
  (bind _returnvalue (`AddComponent|NODE_AddBoxComponent-0` :`RelativeTransform` (`self.Collider`)))
  (`BoxComponent.SetBoxExtent` _returnvalue (`self.ColliderSize`) true))