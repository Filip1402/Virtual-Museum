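; Construction-script Blueprint that builds a procedural array of deformed spline mesh segments along a spline.
; It divides the spline length by Spacing and adds a spline mesh component per step, applying the configurable mesh, material, forward axis and mobility, with collision enabled.
; Each segment takes world-space positions and scaled direction tangents from the spline, with ElementOffset trimming both ends and Offset accumulating per index.
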(fn `UserConstructionScript`
  (bind _spline (`self.Spline`))
  (bind _spacing (`self.Spacing`))
  (bind _tangent_scale (`self.Tangent_scale`))
  (for _index (range (+ (`.ReturnValue` (`KismetMathLibrary.FMod` (`SplineComponent.GetSplineLength` _spline) _spacing)) 1))
    (bind _returnvalue (`AddComponent|NODE_AddSplineMeshComponent-1` :`bManualAttachment` true))
    (`SplineMeshComponent.SetForwardAxis` _returnvalue (`self.Forward axis`) true)
    (`SceneComponent.SetMobility` _returnvalue (`self.Mobility`))
    (`PrimitiveComponent.SetCollisionEnabled` _returnvalue "QueryAndPhysics")
    (`StaticMeshComponent.SetStaticMesh` _returnvalue (`self.Static mesh `))
    (`PrimitiveComponent.SetMaterial` _returnvalue 0 (`self.Material`))
    (bind _returnvalue_2 (* _index _spacing))
    (bind _returnvalue_3 (+ _returnvalue_2 (`self.ElementOffset`)))
    (bind _returnvalue_4 (* (`self.Offset`) _index))
    (bind _returnvalue_5 (- (+ _spacing _returnvalue_2) (`self.ElementOffset`)))
    (`SplineMeshComponent.SetStartAndEnd` _returnvalue (+ (`SplineComponent.GetLocationAtDistanceAlongSpline` _spline _returnvalue_3 "World") _returnvalue_4) (* (`SplineComponent.GetDirectionAtDistanceAlongSpline` _spline _returnvalue_3 "World") _tangent_scale) (+ (`SplineComponent.GetLocationAtDistanceAlongSpline` _spline _returnvalue_5 "World") _returnvalue_4) (* (`SplineComponent.GetDirectionAtDistanceAlongSpline` _spline _returnvalue_5 "World") _tangent_scale) true)))