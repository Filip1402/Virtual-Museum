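; Spline placement actor that fills a spline with repeated copies of a chosen static mesh using a Hierarchical Instanced Static Mesh component.
; The construction script sets the mesh and spaces instances by a custom section length or the mesh's X bounds scaled by the actor.
; It adds one local-space instance per whole section, optionally rotated to follow the spline, then applies collision and the configured mobility.
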(fn `UserConstructionScript`
  (bind _returnvalue_x (`KismetMathLibrary.BreakVector` (`self.GetActorScale3D`)))
  (bind _hierarchicalinstancedstaticmesh (`self.HierarchicalInstancedStaticMesh`))
  (bind _returnvalue (* (`self.Current Index`) (`self.SectionLength`)))
  (bind (_min _max) (break `Box` (`StaticMesh.GetBoundingBox` (`self.MyStaticMesh`))))
  (bind _returnvalue_2 (`SplineComponent.GetLocationAtDistanceAlongSpline` (`self.Spline`) _returnvalue "Local"))
  ;[0 1 0.6953] Defines a section length and the static mesh
  (`StaticMeshComponent.SetStaticMesh` (`self.HierarchicalInstancedStaticMesh`) (`self.MyStaticMesh`)) ; Public Var, individual to each actors
  (set `self.SectionLengthCoef` (- (.x _max) (.x _min)))
  (if (`self.Custom Sencion Length`)
    (set `self.SectionLength` (`self.Custom Section Length`))
    (else
      (set `self.SectionLength` (* _returnvalue_x (`self.SectionLengthCoef`)))))
  ;[0.3828 1 0] For each sections based on the length of the spline divided by the defined section length, add an instance of the static mesh at the desired location following the index times the section length
  (for _index (range (`KismetMathLibrary.FTrunc` (/ (`SplineComponent.GetSplineLength` (`self.Spline`)) (`self.SectionLength`))))
    (set `self.Current Index` _index)
    (if (`self.EnableRotation`)
      (`InstancedStaticMeshComponent.AddInstance` _hierarchicalinstancedstaticmesh (`KismetMathLibrary.MakeTransform` _returnvalue_2 (`SplineComponent.GetRotationAtDistanceAlongSpline` (`self.Spline`) _returnvalue "Local")) false)
      (else
        (`InstancedStaticMeshComponent.AddInstance` _hierarchicalinstancedstaticmesh (`KismetMathLibrary.Conv_VectorToTransform` _returnvalue_2) false)))
    (`PrimitiveComponent.SetCollisionEnabled` _hierarchicalinstancedstaticmesh "QueryAndPhysics")
    (`SceneComponent.SetMobility` _hierarchicalinstancedstaticmesh (`self.Mobility`))))