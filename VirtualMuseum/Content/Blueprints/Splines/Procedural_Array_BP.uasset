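; Procedural array actor that places static mesh components at regular intervals along a spline.
; The construction script divides spline length by Spacing and adds a collision-enabled component at each step, matching the spline's world location and rotation at unit scale.
; Components use manual attachment, so the world-space transforms apply directly.
; The mesh and material setters show no assigned asset, and the event graph is empty.
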(fn `UserConstructionScript`
  (bind _spline (`self.Spline`))
  (bind _spacing (`self.Spacing`))
  (for _index (range (+ (`.ReturnValue` (`KismetMathLibrary.FMod` (`SplineComponent.GetSplineLength` _spline) _spacing)) 1))
    (bind _returnvalue (* _index _spacing))
    (bind _returnvalue_2 (`AddComponent|NODE_AddStaticMeshComponent-0` :`bManualAttachment` true :`RelativeTransform` (`KismetMathLibrary.MakeTransform` (`SplineComponent.GetLocationAtDistanceAlongSpline` _spline _returnvalue "World") (`SplineComponent.GetRotationAtDistanceAlongSpline` _spline _returnvalue "World"))))
    (`PrimitiveComponent.SetCollisionEnabled` _returnvalue_2 "QueryAndPhysics")
    (`StaticMeshComponent.SetStaticMesh` _returnvalue_2 null)
    (`PrimitiveComponent.SetMaterial` _returnvalue_2 0 null)))